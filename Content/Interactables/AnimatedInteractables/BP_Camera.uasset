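; Security camera that sweeps back and forth and compromises the player's stealth while they are inside its detection cone.
; A timeline lerps the Arrow's yaw either side of its starting angle, with a FlipFlop alternating reverse and play for an endless sweep.
; Cone overlaps store or clear the player and adjust their DetectionCount.
; Tick calls StealthCompromised on the stored player with a delta-time-scaled amount.
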(event `self.ReceiveBeginPlay`
  (bind (_relativerotation_roll _relativerotation_pitch _relativerotation_yaw) (`KismetMathLibrary.BreakRotator` (`SceneComponent.RelativeRotation` (`self.Arrow`))))
  ; Camera Pan
  (set `self.MinRotation` (- _relativerotation_yaw 65.0))
  (set `self.MaxRotation` (+ _relativerotation_yaw 65.0))
  (bind (_direction _alpha) (`Timeline|Alpha` :!label _label)
    (:`Update`
      (`SceneComponent.K2_SetRelativeRotation` (`self.Arrow`) (`KismetMathLibrary.MakeRotator` 0.0 0.0 (`KismetMathLibrary.Lerp` (`self.MinRotation`) (`self.MaxRotation`) _alpha)) false false))
    (:`Finished`
      (`self.LoopTimeline`))))

(event `LoopTimeline`
  ; Camera Pan
  (`/Engine/EditorBlueprintResources/StandardMacros.FlipFlop`
    (:`A`
      (goto _label :!via `Reverse`))
    (:`B`
      (goto _label))))

(event `self.Cone.OnComponentBeginOverlap`
  (params (OverlappedComponent :type "PrimitiveComponent Object Reference") (OtherActor :type "Actor Object Reference") (OtherComp :type "PrimitiveComponent Object Reference") (OtherBodyIndex :type Integer) (bFromSweep :type Boolean) (SweepResult :type "HitResult Structure (by ref)"))
  ; Player Detection
  (bind _asbp_player_char (cast `/Game/Player/BP_PlayerChar` OtherActor))
  (set `self.OverlapPlayer` _asbp_player_char)
  (set `/Game/Player/BP_PlayerChar.DetectionCount` (+ (`/Game/Player/BP_PlayerChar.DetectionCount` _asbp_player_char) 1) _asbp_player_char))

(event `self.ReceiveTick`
  (params (DeltaSeconds :type "Float (single-precision)"))
  (bind _overlapplayer (`self.OverlapPlayer`))
  ; Player Detection
  (if (`KismetSystemLibrary.IsValid` _overlapplayer)
    (`/Game/Player/BP_PlayerChar.StealthCompromised` _overlapplayer (* DeltaSeconds 500.0))))

(event `self.Cone.OnComponentEndOverlap`
  (params (OverlappedComponent :type "PrimitiveComponent Object Reference") (OtherActor :type "Actor Object Reference") (OtherComp :type "PrimitiveComponent Object Reference") (OtherBodyIndex :type Integer))
  ; Player Detection
  (bind _asbp_player_char (cast `/Game/Player/BP_PlayerChar` OtherActor))
  (set `self.OverlapPlayer` null)
  (set `/Game/Player/BP_PlayerChar.DetectionCount` (- (`/Game/Player/BP_PlayerChar.DetectionCount` _asbp_player_char) 1) _asbp_player_char))

(fn `UserConstructionScript`
  (locals (ConeColorDMI :type "MaterialInstanceDynamic Object Reference")))