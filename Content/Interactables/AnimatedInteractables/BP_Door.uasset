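; BP_Door is an interactable door that toggles open and closed through the INTInteract event once UnlockCount reaches LockCount.
; A FlipFlop plays or reverses the Alpha timeline, which lerps the yaw of the Arrow component from closed to open.
; On opening, UpdateDoorAngle uses a dot product of the door's forward vector and direction to the player to pick the swing direction.
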(event `/Game/Interfaces/Interface_Interact.INT_Interact`
  (params (PlayerRef :type "/Game/Player/BP_PlayerChar Object Reference"))
  (if (>= (`self.UnlockCount`) (`self.LockCount`))
    (`/Engine/EditorBlueprintResources/StandardMacros.FlipFlop`
      (:`A`
        (bind _returnvalue (`self.UpdateDoorAngle` PlayerRef))
        (bind (_direction _alpha_track) (`Timeline|Alpha` :!label _label)
          (:`Update`
            (`SceneComponent.K2_SetRelativeRotation` (`self.Arrow`) (`KismetMathLibrary.MakeRotator` 0.0 0.0 (`KismetMathLibrary.Lerp` 0.0 _returnvalue _alpha_track)) false false))))
      (:`B`
        (goto _label :!via `Reverse`)))))

(fn `UpdateDoorAngle`
  (params (self2 :type "Actor Object Reference"))
  (returns (ReturnValue :type "Float (double-precision)"))
  (return (select `bool` (> (`KismetMathLibrary.Dot_VectorVector` (`KismetMathLibrary.GetDirectionUnitVector` (`self.K2_GetActorLocation`) (`self.K2_GetActorLocation` self2)) (`self.GetActorForwardVector`)) 0.0) :`false` -90.0 :`true` 90.0)))

(fn `UserConstructionScript`)