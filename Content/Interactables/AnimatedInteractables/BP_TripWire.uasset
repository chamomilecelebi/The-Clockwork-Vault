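; BP_TripWire is a laser trip wire hazard that calls WinLoseCondition with false on the player character when it overlaps the beam's Cylinder.
; The construction script gives the Cylinder a dynamic instance of MAT_ColorGlow and tints it red.
; On BeginPlay, LaserLength is added to the Arrow component's Z scale to set the laser's length.
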(event `self.ReceiveBeginPlay`
  (bind _arrow (`self.Arrow`))
  (`SceneComponent.SetRelativeScale3D` _arrow (+ (`SceneComponent.RelativeScale3D` _arrow) (`KismetMathLibrary.MakeVector` 0.0 0.0 (`self.LaserLength`)))))

(event `self.Cylinder.OnComponentBeginOverlap`
  (params (OverlappedComponent :type "PrimitiveComponent Object Reference") (OtherActor :type "Actor Object Reference") (OtherComp :type "PrimitiveComponent Object Reference") (OtherBodyIndex :type Integer) (bFromSweep :type Boolean) (SweepResult :type "HitResult Structure (by ref)"))
  (bind _asbp_player_char (cast `/Game/Player/BP_PlayerChar` OtherActor))
  (`/Game/Player/BP_PlayerChar.WinLoseCondition` _asbp_player_char false))

(fn `UserConstructionScript`
  (bind _returnvalue (`PrimitiveComponent.CreateDynamicMaterialInstance` (`self.Cylinder`) 0 "/Game/Interactables/AnimatedInteractables/MAT_ColorGlow.MAT_ColorGlow" "None"))
  (bind _output_get (set `self.ColorDMI` _returnvalue))
  (`MaterialInstanceDynamic.SetVectorParameterValue` _output_get "BaseColor" (struct :`R` 1.0 :`A` 1.0)))