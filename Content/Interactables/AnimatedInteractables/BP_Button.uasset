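; BP_Button is a color-coded pressure button that changes the UnlockCount of its TargetDoor.
; A BP_PhysicsPickup of matching PickupColor entering the Overlap component increments the count and plays a timeline that lowers the button mesh.
; Any pickup leaving decrements the count and reverses the timeline, without a color check.
; The construction script tints a dynamic glow material with PickupColor.
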(event `self.Overlap.OnComponentBeginOverlap`
  (params (OverlappedComponent :type "PrimitiveComponent Object Reference") (OtherActor :type "Actor Object Reference") (OtherComp :type "PrimitiveComponent Object Reference") (OtherBodyIndex :type Integer) (bFromSweep :type Boolean) (SweepResult :type "HitResult Structure (by ref)"))
  (bind _targetdoor (`self.TargetDoor`))
  (bind _asbp_physics_pickup (cast `/Game/Interactables/BP_PhysicsPickup` OtherActor))
  (if (== (`/Game/Interactables/BP_PhysicsPickup.PickupColor` _asbp_physics_pickup) (`self.PickupColor`))
    (set `/Game/Interactables/AnimatedInteractables/BP_Door.UnlockCount` (+ (`/Game/Interactables/AnimatedInteractables/BP_Door.UnlockCount` _targetdoor) 1) _targetdoor)
    (bind (_direction _alpha_track) (`Timeline|Alpha` :!label _label)
      (:`Update`
        (`SceneComponent.K2_SetRelativeLocation` (`self.Button`) (`KismetMathLibrary.MakeVector` 0.0 0.0 (`KismetMathLibrary.Lerp` 5.0 1.0 _alpha_track)) false false)))))

(event `self.Overlap.OnComponentEndOverlap`
  (params (OverlappedComponent :type "PrimitiveComponent Object Reference") (OtherActor :type "Actor Object Reference") (OtherComp :type "PrimitiveComponent Object Reference") (OtherBodyIndex :type Integer))
  (bind _targetdoor (`self.TargetDoor`))
  (cast `/Game/Interactables/BP_PhysicsPickup` OtherActor)
  (set `/Game/Interactables/AnimatedInteractables/BP_Door.UnlockCount` (- (`/Game/Interactables/AnimatedInteractables/BP_Door.UnlockCount` _targetdoor) 1) _targetdoor)
  (goto _label :!via `Reverse`))

(fn `UserConstructionScript`
  (bind _returnvalue (`PrimitiveComponent.CreateDynamicMaterialInstance` (`self.Button`) 0 "/Game/Interactables/AnimatedInteractables/MAT_ColorGlow.MAT_ColorGlow" "None"))
  (bind _output_get (set `self.ColorDMI` _returnvalue))
  (`MaterialInstanceDynamic.SetVectorParameterValue` _output_get "BaseColor" (`self.PickupColor`)))